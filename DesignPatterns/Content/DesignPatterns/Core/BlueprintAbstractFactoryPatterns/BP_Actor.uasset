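; BP_Actor is a demo actor for the Abstract Factory design pattern, running its example on BeginPlay.
; It constructs a FactoryHuawei object, asks it to create pad and phone products, and calls ShowInfo on each.
; It then constructs a FactoryApple object but does not create or use any products from it.
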(event EventBeginPlay
  (Utilities|FlowControl|Sequence
    (:then_0
      (bind _returnvalue (Game|ConstructObjectfromClass (Variables|Default|GetFactoryHuawei) self))
      (Utilities|FlowControl|Sequence
        (:then_0
          (bind _huawei (Default|CreateProductPad _returnvalue))
          (Default|ShowInfo _huawei))
        (:then_1
          (bind _newparam (Default|CreateProductPhone _returnvalue))
          (Default|ShowInfo _newparam))))
    (:then_1
      (Game|ConstructObjectfromClass (Variables|Default|GetFactoryApple) self))))

(fn ConstructionScript)